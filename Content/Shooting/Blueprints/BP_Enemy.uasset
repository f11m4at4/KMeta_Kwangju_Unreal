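; BP_Enemy is a shooter enemy that flies in a straight line toward where the player was when it spawned.
; BeginPlay finds BP_Player and caches a normalized direction once, and Tick moves the actor along it by speed and delta time without sweeping.
; When its cube overlaps an actor whose display name lacks "Enemy", it destroys both and plays an explosion effect and sound.
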(event `self.ReceiveBeginPlay`
  ; 타겟을 찾는다.
  (bind _returnvalue (`GameplayStatics.GetActorOfClass` "/Game/Shooting/Blueprints/BP_Player.BP_Player_C"))
  (set `self.Target` _returnvalue)
  (`self.FindDirection`))

(event `self.ReceiveTick`
  (params (DeltaSeconds :type "Float (single-precision)"))
  (`self.Move` DeltaSeconds))

(event `self.Cube.OnComponentBeginOverlap`
  (params (OverlappedComponent :type "PrimitiveComponent Object Reference") (OtherActor :type "Actor Object Reference") (OtherComp :type "PrimitiveComponent Object Reference") (OtherBodyIndex :type Integer) (bFromSweep :type Boolean) (SweepResult :type "HitResult Structure (by ref)"))
  ; 부딪혔을 때 처리
  ;; 적이 아닐때만 너도 죽고나도죽고 처리하자
  (if (not (`KismetStringLibrary.Contains` (`KismetSystemLibrary.GetDisplayName` OtherActor) "Enemy"))
    (`self.K2_DestroyActor` OtherActor)
    (`self.K2_DestroyActor`)
    (`GameplayStatics.SpawnEmitterAtLocation` "/Game/StarterContent/Particles/P_Explosion.P_Explosion" (`self.K2_GetActorLocation`))
    (`GameplayStatics.PlaySound2D` "/Game/Shooting/Explosion.Explosion" 1.0 1.0 0.0 null null)))

(fn `FindDirection`
  ; 방향을 구한다.
  (set `self.Direction` (`KismetMathLibrary.Normal` (- (`self.K2_GetActorLocation` (`self.Target`)) (`self.K2_GetActorLocation`)))))

(fn `Move`
  (params (A :type "Float (single-precision)"))
  ; 이동하고 싶다.
  ;; P
  (`self.K2_SetActorLocation` (+ (* A (* (`self.Direction`) (`self.Speed`))) (`self.K2_GetActorLocation`))))

(fn `UserConstructionScript`)