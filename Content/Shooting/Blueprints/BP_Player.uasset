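; BP_Player is the player of a shooting game, moving on the YZ plane and firing bullets.
; Horizontal and Vertical axis inputs both feed one assignment of the Direction vector, with X fixed at zero.
; Tick moves the actor by Direction, Speed and delta time, without sweeping for collision.
; Pressing Fire spawns a BP_Bullet at the player's location and plays a blaster sound.
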(event `self.ReceiveBeginPlay`)

(event `self.ReceiveTick`
  (params (DeltaSeconds :type "Float (single-precision)"))
  ; 이동하고 싶다.
  ;; P
  (`self.K2_SetActorLocation` (+ (* DeltaSeconds (* (`self.Direction`) (`self.Speed`))) (`self.K2_GetActorLocation`))))

(event `InputAxis|Horizontal`
  (params (AxisValue :type "Float (single-precision)"))
  ; 방향구하기
  (set `self.Direction` (`KismetMathLibrary.MakeVector` 0.0 AxisValue (stale `InputAxis|Vertical` AxisValue)) :!label _label))

(event `InputAxis|Vertical`
  (params (AxisValue :type "Float (single-precision)"))
  ; 방향구하기
  (goto _label))

(event `InputAction|Fire`
  (params (Key :type "Key Structure"))
  ; 총알을 발사하고 싶다.
  (:`Pressed`
    (`|SpawnActorFromClass` "/Game/Shooting/Blueprints/BP_Bullet.BP_Bullet_C" (`KismetMathLibrary.MakeTransform` (`self.K2_GetActorLocation`)) "Undefined" "MultiplyWithRoot" null null)
    (`GameplayStatics.PlaySound2D` "/Game/Shooting/star-wars-blaster.star-wars-blaster" 1.0 1.0 0.0 null null)))

(fn `UserConstructionScript`)